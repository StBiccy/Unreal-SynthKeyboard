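; Synth manager that bridges an on-screen Keyboard widget and a MetaSound-style Korg Mono/Poly synthesizer audio component, MSKorgMonopoly.
; On BeginPlay it creates the widget, shows the mouse cursor and enables game-and-UI input.
; Custom events forward values as named sound parameters: MIDI note plus trigger, volume, four VCOs, noise, pulse width and modulation, filter, and both ADSR envelopes.
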(event Custom|Trigger
  (params (Midi%20Val :type Float%20%28double-precision%29))
  (bind _ms_korgmonopoly (Variables|Default|GetMS_KorgMonopoly))
  ;[1 1 1] Key Trigger
  (Audio|Parameter|SetFloatParameter _ms_korgmonopoly "MIDI Input" Midi%20Val :!class /Script/AudioExtensions.AudioParameterControllerInterface)
  (Class|AudioParameterControllerInterface|SetTriggerParameter _ms_korgmonopoly "Trigger"))

(event Custom|volume%20change
  (params (value :type Float%20%28double-precision%29))
  ;[1 1 1] Volume Change
  (Audio|Parameter|SetFloatParameter (Variables|Default|GetMS_KorgMonopoly) "Volume" value :!class /Script/AudioExtensions.AudioParameterControllerInterface))

(event Custom|ChangeVCO2
  (params (Wave :type Integer) (Oct :type Integer) (Level :type Float%20%28double-precision%29))
  (bind _ms_korgmonopoly (Variables|Default|GetMS_KorgMonopoly))
  ;[1 1 1] VCOs
  (Effects|Components|ParticleSystem|SetIntParameter _ms_korgmonopoly "VCO2Wave" Wave)
  (Effects|Components|ParticleSystem|SetIntParameter _ms_korgmonopoly "Octive Range 2" Oct)
  (Audio|Parameter|SetFloatParameter _ms_korgmonopoly "VCO 2 Level" Level :!class /Script/AudioExtensions.AudioParameterControllerInterface))

(event Custom|ChangePWM
  (params (PWMI :type Float%20%28double-precision%29))
  (Audio|Parameter|SetFloatParameter (Variables|Default|GetMS_KorgMonopoly) "Pusle WIdth Mudulation" (* PWMI 5.0) :!class /Script/AudioExtensions.AudioParameterControllerInterface))

(event Custom|ChangeNoise
  (params (Level :type Float%20%28double-precision%29))
  (Audio|Parameter|SetFloatParameter (Variables|Default|GetMS_KorgMonopoly) "Noise Level" Level :!class /Script/AudioExtensions.AudioParameterControllerInterface))

(event Custom|ChangePW
  (params (PW :type Float%20%28double-precision%29))
  (Audio|Parameter|SetFloatParameter (Variables|Default|GetMS_KorgMonopoly) "PuseWidth" PW :!class /Script/AudioExtensions.AudioParameterControllerInterface))

(event Custom|VCF%20EG%20Change
  (params (attack :type Float%20%28double-precision%29) (decay :type Float%20%28double-precision%29) (sustain :type Float%20%28double-precision%29) (release :type Float%20%28double-precision%29))
  (bind _ms_korgmonopoly (Variables|Default|GetMS_KorgMonopoly))
  ;[1 1 1] VCF EG
  (Audio|Parameter|SetFloatParameter _ms_korgmonopoly "VCF EG Attack" attack :!class /Script/AudioExtensions.AudioParameterControllerInterface)
  (Audio|Parameter|SetFloatParameter _ms_korgmonopoly "VCF EG Decay" decay :!class /Script/AudioExtensions.AudioParameterControllerInterface)
  (Audio|Parameter|SetFloatParameter _ms_korgmonopoly "VCF EG Sustain" sustain :!class /Script/AudioExtensions.AudioParameterControllerInterface)
  (Audio|Parameter|SetFloatParameter _ms_korgmonopoly "VCF EG Relase" release :!class /Script/AudioExtensions.AudioParameterControllerInterface))

(event Custom|ChangeVCO3
  (params (Wave :type Integer) (Oct :type Integer) (Level :type Float%20%28double-precision%29))
  (bind _ms_korgmonopoly (Variables|Default|GetMS_KorgMonopoly))
  ;[1 1 1] VCOs
  (Effects|Components|ParticleSystem|SetIntParameter _ms_korgmonopoly "VCO3Wave" Wave)
  (Effects|Components|ParticleSystem|SetIntParameter _ms_korgmonopoly "Octive Range 3" Oct)
  (Audio|Parameter|SetFloatParameter _ms_korgmonopoly "VCO 3 Level" Level :!class /Script/AudioExtensions.AudioParameterControllerInterface))

(event Custom|VCF%20Change
  (params (Cutoff :type Float%20%28double-precision%29) (Resonance :type Float%20%28double-precision%29))
  (bind _ms_korgmonopoly (Variables|Default|GetMS_KorgMonopoly))
  ;[1 1 1] VCF
  (Audio|Parameter|SetFloatParameter _ms_korgmonopoly "VCF Cutoff" Cutoff :!class /Script/AudioExtensions.AudioParameterControllerInterface)
  (Audio|Parameter|SetFloatParameter _ms_korgmonopoly "VCF Resonance" Resonance :!class /Script/AudioExtensions.AudioParameterControllerInterface))

(event Custom|ChangeVCO0
  (params (Wave :type Integer) (Oct :type Integer) (Level :type Float%20%28double-precision%29))
  (bind _ms_korgmonopoly (Variables|Default|GetMS_KorgMonopoly))
  ;[1 1 1] VCOs
  (Effects|Components|ParticleSystem|SetIntParameter _ms_korgmonopoly "VCO0Wave" Wave)
  (Effects|Components|ParticleSystem|SetIntParameter _ms_korgmonopoly "Octive Range 0" Oct)
  (Audio|Parameter|SetFloatParameter _ms_korgmonopoly "VCO 0 Level" Level :!class /Script/AudioExtensions.AudioParameterControllerInterface))

(event Custom|ChangeVCO1
  (params (Wave :type Integer) (Oct :type Integer) (Level :type Float%20%28double-precision%29))
  (bind _ms_korgmonopoly (Variables|Default|GetMS_KorgMonopoly))
  ;[1 1 1] VCOs
  (Effects|Components|ParticleSystem|SetIntParameter _ms_korgmonopoly "VCO1Wave" Wave)
  (Effects|Components|ParticleSystem|SetIntParameter _ms_korgmonopoly "Octive Range 1" Oct)
  (Audio|Parameter|SetFloatParameter _ms_korgmonopoly "VCO 1 Level" Level :!class /Script/AudioExtensions.AudioParameterControllerInterface))

(event Custom|VCA%20EG%20Change
  (params (Attack :type Float%20%28double-precision%29) (Decay :type Float%20%28double-precision%29) (Sustain :type Float%20%28double-precision%29) (Relase :type Float%20%28double-precision%29))
  (bind _ms_korgmonopoly (Variables|Default|GetMS_KorgMonopoly))
  ;[1 1 1] VCA EG
  (Audio|Parameter|SetFloatParameter _ms_korgmonopoly "VCA EG Attack" Attack :!class /Script/AudioExtensions.AudioParameterControllerInterface)
  (Audio|Parameter|SetFloatParameter _ms_korgmonopoly "VCA EG Decay" Decay :!class /Script/AudioExtensions.AudioParameterControllerInterface)
  (Audio|Parameter|SetFloatParameter _ms_korgmonopoly "VCA EG Sustain" Sustain :!class /Script/AudioExtensions.AudioParameterControllerInterface)
  (Audio|Parameter|SetFloatParameter _ms_korgmonopoly "VCA EG Relase" Relase :!class /Script/AudioExtensions.AudioParameterControllerInterface))

(event EventBeginPlay
  (bind _returnvalue (Game|GetPlayerController 0))
  ;[1 1 1] Construct
  (bind _returnvalue_2 (UserInterface|CreateWidget "/Game/Keyboard.Keyboard_C"))
  (bind _output_get (Variables|Default|SetUI _returnvalue_2))
  (UserInterface|Viewport|AddtoViewport _output_get 0)
  (Input|SetInputModeGameandUI _returnvalue _output_get "DoNotLock" true false)
  (Variables|/Script/Engine.PlayerController|SetbShowMouseCursor _returnvalue true)
  (Input|EnableInput _returnvalue)
  (UserInterface|Viewport|AddtoViewport (Variables|Default|GetUI) 0))

(fn ConstructionScript)